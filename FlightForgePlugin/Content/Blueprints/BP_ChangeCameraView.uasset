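; Input actor that switches the player's view between drone pawns, a free spectator camera and a 360 pawn.
; Pressing N possesses each DronePawn in turn, then spawns a SpectatorPawn at its last saved transform and possesses it.
; Leaving spectator mode saves that transform and destroys the spectator pawn.
; Pressing K possesses the first BP_360 actor found in the level.
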(event `self.ReceiveBeginPlay`
  (`self.EnableInput` (`GameplayStatics.GetPlayerController` 0)))

(event `Key|N`
  (params (Key :type "Key Structure"))
  (bind _returnvalue (`GameplayStatics.GetPlayerController` 0))
  (bind _dronetopossesid (`self.DronetoPossesID`))
  ;[1 1 1] Change Camera View
  (:`Pressed`
    (bind _returnvalue_2 (`GameplayStatics.GetActorOfClass` "/Script/Engine.SpectatorPawn"))
    (if (`KismetSystemLibrary.IsValid` _returnvalue_2)
      (set `self.LastSpectatorPOS` (`self.GetTransform` _returnvalue_2))
      (`self.K2_DestroyActor` _returnvalue_2))
    (bind _outactors (`GameplayStatics.GetAllActorsOfClass` "/Script/ueds.DronePawn"))
    (if (< _dronetopossesid (`KismetArrayLibrary.Array_Length` _outactors))
      (`Controller.Possess` _returnvalue (`|GetArrayItem` _outactors _dronetopossesid))
      (set `self.DronetoPossesID` (+ _dronetopossesid 1))
      (else
        (set `self.DronetoPossesID` 0)
        (bind _returnvalue_3 (`|SpawnActorFromClass` "/Script/Engine.SpectatorPawn" (`self.LastSpectatorPOS`) "AlwaysSpawn" "MultiplyWithRoot" null null))
        (`Controller.Possess` _returnvalue _returnvalue_3)))))

(event `Key|K`
  (params (Key :type "Key Structure"))
  (:`Pressed`
    (bind _returnvalue (`GameplayStatics.GetActorOfClass` "/Game/Blueprints/BP_360.BP_360_C"))
    (`Controller.Possess` (`GameplayStatics.GetPlayerController` 0) _returnvalue)))

(fn `UserConstructionScript`)