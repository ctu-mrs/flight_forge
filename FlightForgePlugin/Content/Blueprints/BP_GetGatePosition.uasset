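; BP_GetGatePosition exports the positions and headings of the race gates in the level to a CSV file on BeginPlay.
; It gathers all BP_a2rl_gate_slim and BP_a2rl_gate_slim_core actors, recording name, location relative to PlayerStart and yaw for each.
; Locations become right-handed metres by scaling and flipping Y, and yaw is negated into a positive-degree heading.
; WriteGateTransformToCsv writes the arrays and its result string is printed.
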(event `self.ReceiveBeginPlay`
  (bind _position_to_print (`self.position to print`))
  (bind _names_to_print (`self.names to print`))
  (bind _returnvalue (`GameplayStatics.GetActorOfClass` "/Script/Engine.PlayerStart"))
  (bind _outactors (`GameplayStatics.GetAllActorsOfClass` "/Game/Worlds/Warehouse/Blueprints/BP_a2rl_gate_slim.BP_a2rl_gate_slim_C"))
  (for _array_element _outactors
    ;[1 1 1] Transformation from UE coord to Right-Hand cordinates
    (`KismetArrayLibrary.Array_Add` (`self.position to print`) (/ (- (`self.K2_GetActorLocation` _array_element) (`self.K2_GetActorLocation` _returnvalue)) (100.0 -100.0 100.0)))
    (`KismetArrayLibrary.Array_Add` (`self.names to print`) (`KismetSystemLibrary.GetDisplayName` _array_element))
    (bind _returnvalue_2 (`self.GetTransform` _array_element))
    (if (<= (.yaw (.rotation _returnvalue_2)) 0.0)
      (`KismetArrayLibrary.Array_Add` (`self.heading to print`) (* (.yaw (.rotation _returnvalue_2)) -1.0))
      (else
        (`KismetArrayLibrary.Array_Add` (`self.heading to print`) (- 360.0 (.yaw (.rotation _returnvalue_2)))))))
  (bind _outactors_2 (`GameplayStatics.GetAllActorsOfClass` "/Game/Worlds/Warehouse/Blueprints/BP_a2rl_gate_slim_core.BP_a2rl_gate_slim_core_C"))
  (for _array_element_2 _outactors_2
    (`KismetArrayLibrary.Array_Add` _position_to_print (/ (- (`self.K2_GetActorLocation` _array_element_2) (`self.K2_GetActorLocation` _returnvalue)) (100.0 -100.0 100.0)))
    (`KismetArrayLibrary.Array_Add` _names_to_print (`KismetSystemLibrary.GetDisplayName` _array_element_2))
    (bind _returnvalue_3 (`self.GetTransform` _array_element_2))
    (if (<= (.yaw (.rotation _returnvalue_3)) 0.0)
      (`KismetArrayLibrary.Array_Add` (`self.heading to print`) (* (.yaw (.rotation _returnvalue_3)) -1.0))
      (else
        (`KismetArrayLibrary.Array_Add` (`self.heading to print`) (- 360.0 (.yaw (.rotation _returnvalue_3)))))))
  (bind (_boutresult _outstring) (`BlueprintUtils.WriteGateTransformToCsv` "Race_2_Gate_Position" _names_to_print _position_to_print (`self.heading to print`)))
  (`KismetSystemLibrary.PrintString` _outstring))

(fn `UserConstructionScript`)